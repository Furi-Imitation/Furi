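; BP_BlownAway2 is a looping dissolve effect that pairs a skeletal mesh with a Niagara particle system.
; BeginPlay calls Dissolve, which waits briefly, activates Niagara and plays a timeline.
; The timeline drives a VisibilityLevel scalar parameter on the mesh materials through a lerp, sweeping the dissolve across the mesh.
; When it finishes, Niagara deactivates and Dissolve calls itself again after a delay, repeating indefinitely.
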(event `self.ReceiveBeginPlay`
  (`self.Dissolve`))

(event `Dissolve`
  (`KismetSystemLibrary.Delay` 1.0)
  (`ActorComponent.Activate` (`self.Niagara`) true)
  (bind (_direction _newtrack_0) (`Timeline|Timeline_0` :!via `PlayFromStart`)
    (:`Update`
      (`MeshComponent.SetScalarParameterValueOnMaterials` (`self.SkeletalMesh`) "VisibilityLevel" (`KismetMathLibrary.Lerp` -100.0 200.0 _newtrack_0)))
    (:`Finished`
      (`ActorComponent.Deactivate` (`self.Niagara`))
      (`KismetSystemLibrary.Delay` 1.0)
      (`self.Dissolve`))))

(fn `UserConstructionScript`)