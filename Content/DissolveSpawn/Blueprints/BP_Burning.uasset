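; BP_Burning is a looping effect actor that sets its mesh on fire and then dissolves it, accompanied by Niagara fire and ash.
; A Burning timeline raises the material FireAmount and fire spawn rate, then a delayed Dissolve timeline raises the Amount parameter while tapering the fire as ash activates.
; After a pause it resets both material parameters and calls Begin again, repeating endlessly from BeginPlay.
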(event `self.ReceiveBeginPlay`
  (`self.Begin`))

(event `Begin`
  (bind _mesh (`self.Mesh`))
  (`ActorComponent.Activate` (`self.Fire`) false)
  (bind (_direction _newtrack_0) (`Timeline|Burning` :!via `PlayFromStart`)
    (:`Update`
      (`MeshComponent.SetScalarParameterValueOnMaterials` (`self.Mesh`) "FireAmount" _newtrack_0)
      (`FXSystemComponent.SetFloatParameter` (`self.Fire`) "SpawnRate" (`KismetMathLibrary.Lerp` 0.0 500.0 _newtrack_0)))
    (:`Finished`
      (`KismetSystemLibrary.Delay` 2.0)
      (`ActorComponent.Activate` (`self.NS_Ash`) false)
      (bind (_direction_2 _newtrack_0_2) (`Timeline|Dissolve` :!via `PlayFromStart`)
        (:`Update`
          (`MeshComponent.SetScalarParameterValueOnMaterials` (`self.Mesh`) "Amount" _newtrack_0_2)
          (`FXSystemComponent.SetFloatParameter` (`self.Fire`) "SpawnRate" (`KismetMathLibrary.Lerp` 500.0 0.0 _newtrack_0_2)))
        (:`Finished`
          (`KismetSystemLibrary.Delay` 2.0)
          (`MeshComponent.SetScalarParameterValueOnMaterials` _mesh "FireAmount" 0.0)
          (`MeshComponent.SetScalarParameterValueOnMaterials` _mesh "Amount" 0.0)
          (`self.Begin`))))))

(fn `UserConstructionScript`)