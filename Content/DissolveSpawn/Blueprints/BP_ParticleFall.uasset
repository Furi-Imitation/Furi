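; BP_ParticleFall plays a looping dissolve-spawn effect on a skeletal mesh, paired with a Niagara particle system.
; BeginPlay activates Niagara and starts a timeline that lerps the "Amount" scalar parameter on the mesh's materials.
; When the timeline finishes, Niagara deactivates, then after a short delay both the particles and the timeline restart, repeating indefinitely.
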(event `self.ReceiveBeginPlay`
  (`self.BeginEvent`))

(event `BeginEvent`
  (`ActorComponent.Activate` (`self.Niagara`) true :!label _label)
  (bind (_direction _newtrack_0) (`Timeline|Timeline_0` :!via `PlayFromStart`)
    (:`Update`
      (`MeshComponent.SetScalarParameterValueOnMaterials` (`self.SkeletalMesh`) "Amount" (`KismetMathLibrary.Lerp` 1.1 0.0 _newtrack_0)))
    (:`Finished`
      (`ActorComponent.Deactivate` (`self.Niagara`))
      (`KismetSystemLibrary.Delay` 2.0)
      (goto _label))))

(fn `UserConstructionScript`)