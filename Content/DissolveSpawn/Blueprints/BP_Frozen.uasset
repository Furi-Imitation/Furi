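; BP_Frozen is a looping showcase effect that freezes a skeletal mesh, starting on BeginPlay.
; A first timeline drives the IceAmount material parameter while ramping the Snow particle spawn rate.
; After a pause, SnowBurst fires and a second timeline drives the Amount parameter, likely a dissolve.
; Snow then stops, and after another pause both parameters reset and BeginEvent calls itself to repeat.
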(event `self.ReceiveBeginPlay`
  (`self.BeginEvent`))

(event `BeginEvent`
  (bind _skeletalmesh (`self.SkeletalMesh`))
  (`ActorComponent.Activate` (`self.Snow`) false)
  (bind (_direction _newtrack_0) (`Timeline|Timeline_0` :!via `PlayFromStart`)
    (:`Update`
      (`MeshComponent.SetScalarParameterValueOnMaterials` (`self.SkeletalMesh`) "IceAmount" _newtrack_0)
      (`FXSystemComponent.SetFloatParameter` (`self.Snow`) "SpawnRate" (`KismetMathLibrary.Lerp` 0.0 500.0 _newtrack_0)))
    (:`Finished`
      (`KismetSystemLibrary.Delay` 2.0)
      (`ActorComponent.Activate` (`self.SnowBurst`) false)
      (bind (_direction_2 _newtrack_0_2) (`Timeline|Timeline_1` :!via `PlayFromStart`)
        (:`Update`
          (`MeshComponent.SetScalarParameterValueOnMaterials` (`self.SkeletalMesh`) "Amount" _newtrack_0_2))
        (:`Finished`
          (`ActorComponent.Deactivate` (`self.Snow`))
          (`KismetSystemLibrary.Delay` 2.0)
          (`MeshComponent.SetScalarParameterValueOnMaterials` _skeletalmesh "IceAmount" 0.0)
          (`MeshComponent.SetScalarParameterValueOnMaterials` _skeletalmesh "Amount" 0.0)
          (`self.BeginEvent`))))))

(fn `UserConstructionScript`)