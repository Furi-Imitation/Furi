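; BP_Morph1 runs a looping morph effect, pairing the NSMorph effect component with two timelines.
; On BeginPlay it passes itself to NSMorph as "CallBack" and activates it, then after a delay plays both timelines together to drive Amount1 and Amount2 in the MPC_Morph material parameter collection.
; When the second timeline finishes, it deactivates the effect, resets both parameters after a pause, waits again and restarts.
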(event `self.ReceiveBeginPlay`
  (`NiagaraComponent.SetVariableObject` (`self.NS_Morph`) "CallBack" self :!label _label)
  (`ActorComponent.SetActive` (`self.NS_Morph`) true false)
  (`KismetSystemLibrary.Delay` 4.0)
  (`|ExecutionSequence`
    (:`then_0`
      (bind (_direction _newtrack_0) (`Timeline|Timeline_0` :!via `PlayFromStart`)
        (:`Update`
          (`KismetMaterialLibrary.SetScalarParameterValue` "/Game/DissolveSpawn/Materials/Parametercollection/MPC_Morph.MPC_Morph" "Amount1" _newtrack_0))))
    (:`then_1`
      (bind (_direction_2 _newtrack_0_2) (`Timeline|Timeline_1` :!via `PlayFromStart`)
        (:`Update`
          (`KismetMaterialLibrary.SetScalarParameterValue` "/Game/DissolveSpawn/Materials/Parametercollection/MPC_Morph.MPC_Morph" "Amount2" _newtrack_0_2))
        (:`Finished`
          (`ActorComponent.SetActive` (`self.NS_Morph`) false false)
          (`KismetSystemLibrary.Delay` 5.0)
          (`KismetMaterialLibrary.SetScalarParameterValue` "/Game/DissolveSpawn/Materials/Parametercollection/MPC_Morph.MPC_Morph" "Amount1" 1.0)
          (`KismetMaterialLibrary.SetScalarParameterValue` "/Game/DissolveSpawn/Materials/Parametercollection/MPC_Morph.MPC_Morph" "Amount2")
          (`KismetSystemLibrary.Delay` 3.0)
          (goto _label))))))

(fn `UserConstructionScript`)